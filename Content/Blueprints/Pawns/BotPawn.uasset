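; Bot pawn that wanders to random points until it spots a Character through PawnSensing.
; Seeing a Character sets SeePlayer, which is exposed through Canseeplayer, never cleared here, and stops Tick from starting new moves.
; Tick starts AIMoveTo when the bot is idle, and a one-second delay loop reissues it with new points without rechecking SeePlayer.
; An AIMoveTo targeting the seen Character is unconnected, so no chase runs.
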(event OnSeePawn(PawnSensing)
  (params (Pawn :type Pawn%20Object%20Reference))
  ;[1 1 1] Cuando el Bot puede ver al player
  (bind _ascharacter (Utilities|Casting|CastToCharacter Pawn)
    (:then
      (Variables|Default|SetseePlayer true))
    (:CastFailed
      (Development|PrintString 0 "fallo"))))

(event EventTick
  (params (DeltaSeconds :type Float%20%28single-precision%29))
  ;[1 1 1] Cuando el bot no puede verlo
  (if (not (Variables|Default|GetseePlayer))
    (if (not (Variables|Default|GetbotMoving))
      (AI|AIMoveTo "0" self (Class|NavigationSystem|GetRandomPoint "WorldContext") 0 0.0 false :!label _label
        (:then
          (Variables|Default|SetbotMoving true)
          (Utilities|FlowControl|Delay 0 1.0)
          (goto _label))
        (:OnSuccess
          _)
        (:OnFail
          _))
      (Variables|Default|SetbotMoving false))))

(fn ConstructionScript)

(fn Canseeplayer
  (return (Variables|Default|GetseePlayer)))